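; BP_ModularPlayerController is a player controller whose Possess and IA_Inventory events are empty, so its UI logic is currently disconnected.
; An unreachable chain toggles the resizable inventory window via FlipFlop on the possessed BP_MPC_Character_Master's inventory component, then switches input mode.
; Another unreachable chain creates a right-click context menu widget at high viewport Z-order for locally controlled pawns.
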(event `self.ReceivePossess`
  (params (PossessedPawn :type "Pawn Object Reference")))

(event `EnhancedInput|/ModularPlayerController/Input/Common/Inventory/IA_Inventory`
  (params (ActionValue :type Boolean) (ElapsedSeconds :type "Float (double-precision)") (TriggeredSeconds :type "Float (double-precision)") (InputAction :type "InputAction Object Reference" :default "/ModularPlayerController/Input/Common/Inventory/IA_Inventory.IA_Inventory")))

(fn `UserConstructionScript`)